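; Player spaceship for a shooter, using Enhanced Input for planar movement and timer-throttled firing with sound.
; Each shot spawns bullets in a fan whose count and spacing derive from FireType in the game instance.
; Overlapping tagged power-ups raises FireType, then resets it after a delay.
; Enemy bullet hits decrement Live in the game instance, and the ship is destroyed with an explosion sound at zero.
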(event Custom|Fire_Update
  ;[1 1 1] Fire_Push
  (Variables|Default|SetFire_tempo true))

(event Input|EnhancedActionEvents|EnhancedInputActionBP_Input_Move
  (params (ActionValue :type Vector%202D%20Structure) (ElapsedSeconds :type Float%20%28double-precision%29) (TriggeredSeconds :type Float%20%28double-precision%29) (InputAction :type Input%20Action%20Object%20Reference :default "/Game/assets/Blueprint_Game/BP_Input_Move.BP_Input_Move"))
  (Pawn|Input|AddMovementInput "1.000000,0.000000,0.000000" (.y ActionValue) false)
  (Pawn|Input|AddMovementInput "0.000000,1.000000,0.000000" (.x ActionValue) false))

(event Input|EnhancedActionEvents|EnhancedInputActionBP_Input_Fire
  (params (ActionValue :type Boolean) (ElapsedSeconds :type Float%20%28double-precision%29) (TriggeredSeconds :type Float%20%28double-precision%29) (InputAction :type Input%20Action%20Object%20Reference :default "/Game/assets/Blueprint_Game/BP_Input_Fire.BP_Input_Fire"))
  ;[1 1 1] Fire_Push
  (if (Variables|Default|GetFire_tempo)
    (Audio|PlaySound2D "/Game/Sounds/Mono/Single_Space_Shot.Single_Space_Shot" 0.5 1.0 0.0 0 0)
    (Audio|PlaySound2D "/Game/Sounds/Mono/Plasma_Impact.Plasma_Impact" 1.0 1.0 0.0 0 0)
    (CallFunction|SpawBulletPlayer)
    (Variables|Default|SetFire_tempo false)
    (Utilities|Time|SetTimerbyEvent (delegate Custom|Fire_Update) (Variables|Default|GetTime_Bullet))))

(event EventBeginPlay
  (bind _asplayer_controller (Utilities|Casting|CastToPlayerController (Pawn|GetController)))
  (Utilities|IsValid (PlayerController|LocalPlayerSubsystems|GetEnhancedInputLocalPlayerSubsystem _asplayer_controller)
    (:Is%20Valid
      (Input|AddMappingContext (PlayerController|LocalPlayerSubsystems|GetEnhancedInputLocalPlayerSubsystem _asplayer_controller) "/Game/assets/Blueprint_Game/Bp_Intput_Mapping.Bp_Intput_Mapping" 0 "(bIgnoreAllPressedKeysUntilRelease=True,bForceImmediately=False,bNotifyUserSettings=False)"))))

(event Collision|EventActorBeginOverlap
  (params (OtherActor :type Actor%20Object%20Reference))
  (if (Utilities|Array|ContainsItem (Variables|/Script/Engine.Actor|GetTags OtherActor) "PowerUp_1")
    (bind _asbp_game_instance_shooter (Utilities|Casting|CastToBp_GameInstance_Shooter (Game|GetGameInstance)))
    (Variables|/Game/assets/Blueprint_Game/Bp_GameInstance_Shooter.Bp_GameInstance_Shooter_C|SetFire_type _asbp_game_instance_shooter 2)
    (Utilities|FlowControl|Delay 5.0)
    (CallFunction|ResetVarBullet)
    (elif (Utilities|Array|ContainsItem (Variables|/Script/Engine.Actor|GetTags OtherActor) "PowerUp_2")
      (bind _asbp_game_instance_shooter_2 (Utilities|Casting|CastToBp_GameInstance_Shooter (Game|GetGameInstance)))
      (Variables|/Game/assets/Blueprint_Game/Bp_GameInstance_Shooter.Bp_GameInstance_Shooter_C|SetFire_type _asbp_game_instance_shooter_2 3)
      (Utilities|FlowControl|Delay 5.0)
      (CallFunction|ResetVarBullet)
      (elif (Utilities|Array|ContainsItem (Variables|/Script/Engine.Actor|GetTags OtherActor) "PowerUp_3")
        (bind _asbp_game_instance_shooter_3 (Utilities|Casting|CastToBp_GameInstance_Shooter (Game|GetGameInstance)))
        (Variables|/Game/assets/Blueprint_Game/Bp_GameInstance_Shooter.Bp_GameInstance_Shooter_C|SetFire_type _asbp_game_instance_shooter_3 4)
        (Utilities|FlowControl|Delay 5.0)
        (CallFunction|ResetVarBullet)
        (elif (Utilities|Array|ContainsItem (Variables|/Script/Engine.Actor|GetTags OtherActor) "Bullet_Enemy")
          (bind _asbp_game_instance_shooter_4 (Utilities|Casting|CastToBp_GameInstance_Shooter (Game|GetGameInstance)))
          (bind _output_get (Variables|/Game/assets/Blueprint_Game/Bp_GameInstance_Shooter.Bp_GameInstance_Shooter_C|SetLive _asbp_game_instance_shooter_4 (- (Variables|/Game/assets/Blueprint_Game/Bp_GameInstance_Shooter.Bp_GameInstance_Shooter_C|GetLive _asbp_game_instance_shooter_4) 1)))
          (Utilities|FlowControl|Delay 0.2)
          (if (== _output_get 0)
            (Actor|DestroyActor)
            (Audio|PlaySound2D "/Game/StarterContent/Audio/Explosion01.Explosion01" 2.0 1.0 0.0 0 0)))))))

(event EventTick
  (params (DeltaSeconds :type Float%20%28single-precision%29)))

(fn ConstructionScript)

(fn SpawBulletPlayer
  (bind _asbp_game_instance_shooter (Utilities|Casting|CastToBp_GameInstance_Shooter (Game|GetGameInstance)))
  (if (!= (Variables|/Game/assets/Blueprint_Game/Bp_GameInstance_Shooter.Bp_GameInstance_Shooter_C|GetFire_type _asbp_game_instance_shooter) 0)
    (bind _output_get (Variables|/Game/assets/Blueprint_Game/Bp_GameInstance_Shooter.Bp_GameInstance_Shooter_C|Setrotator_bullet _asbp_game_instance_shooter -15.0)))
  (for _index (range 0 (+ (Variables|/Game/assets/Blueprint_Game/Bp_GameInstance_Shooter.Bp_GameInstance_Shooter_C|GetFire_type _asbp_game_instance_shooter) 0))
    (Game|SpawnActorfromClass "/Game/assets/Blueprints_actors/Bullet1.Bullet1_C" (Math|Transform|MakeTransform (.location (Transformation|GetWorldTransform (Variables|Default|Getspawn_point_fire_1))) (Math|Rotator|CombineRotators (Math|Rotator|MakeRotator 0.0 0.0 _output_get) (Math|Rotator|MakeRotator 0.0 0.0 (* _index (/ 30 (Variables|/Game/assets/Blueprint_Game/Bp_GameInstance_Shooter.Bp_GameInstance_Shooter_C|GetFire_type _asbp_game_instance_shooter))))) "1.000000,1.000000,1.000000") "AlwaysSpawn" "MultiplyWithRoot" 0 0)))

(fn SelectorBullet
  (bind _asbp_game_instance_shooter (Utilities|Casting|CastToBp_GameInstance_Shooter (Game|GetGameInstance))
    (:then
      (if (not (Variables|/Game/assets/Blueprint_Game/Bp_GameInstance_Shooter.Bp_GameInstance_Shooter_C|GetPowerUp_1 _asbp_game_instance_shooter))
        (return (Utilities|Select :Index (Variables|/Game/assets/Blueprint_Game/Bp_GameInstance_Shooter.Bp_GameInstance_Shooter_C|Getlist _asbp_game_instance_shooter) :Option%200 (Variables|Default|GetClass-base) :Option%201 "/Game/assets/Blueprints_actors/Bullet1.Bullet1_C"))))
    (:CastFailed
      (return (Utilities|Select :Index (Variables|/Game/assets/Blueprint_Game/Bp_GameInstance_Shooter.Bp_GameInstance_Shooter_C|Getlist _asbp_game_instance_shooter) :Option%200 (Variables|Default|GetClass-base) :Option%201 "/Game/assets/Blueprints_actors/Bullet1.Bullet1_C")))))

(fn PowerUpSelect
  (params (self2 :type Actor%20Object%20Reference) (self3 :type Actor%20Object%20Reference) (self4 :type Actor%20Object%20Reference)))

(fn ResetVarBullet
  (bind _asbp_game_instance_shooter (Utilities|Casting|CastToBp_GameInstance_Shooter (Game|GetGameInstance)))
  (Variables|/Game/assets/Blueprint_Game/Bp_GameInstance_Shooter.Bp_GameInstance_Shooter_C|SetFire_type _asbp_game_instance_shooter 0)
  (Variables|/Game/assets/Blueprint_Game/Bp_GameInstance_Shooter.Bp_GameInstance_Shooter_C|Setrotator_bullet _asbp_game_instance_shooter 0.0))