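; Timed enemy spawner actor that waits 100 seconds after BeginPlay, then spawns BP_Enemy_2 on a looping four-second timer.
; Each spawn uses a random reachable navmesh point within a large radius around the spawner.
; Tick accumulates elapsed time in Contador, including the initial delay.
; Once it reaches 200 seconds, the next timer call sets VariableEnd on Bp_GameInstance_Shooter and destroys the spawner.
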(event Custom|SpawnEnemy
  (if (< (Variables|Default|GetContador) 2e+02)
    (Game|SpawnActorfromClass "/Game/assets/Blueprints_actors/BP_Enemy_2.BP_Enemy_2_C" (Math|Transform|MakeTransform (.RandomLocation (AI|Navigation|GetRandomReachablePointinRadius (Transformation|GetActorLocation) 6e+03 0 0)) (Transformation|GetActorRotation) "1.000000,1.000000,1.000000") "AlwaysSpawn" "MultiplyWithRoot" 0 0)
    (else
      (bind _asbp_game_instance_shooter (Utilities|Casting|CastToBp_GameInstance_Shooter (Game|GetGameInstance)))
      (Variables|/Game/assets/Blueprint_Game/Bp_GameInstance_Shooter.Bp_GameInstance_Shooter_C|SetVariable_End _asbp_game_instance_shooter true)
      (Actor|DestroyActor))))

(event EventBeginPlay
  (Utilities|FlowControl|Delay 1e+02)
  (Utilities|Time|SetTimerbyEvent (delegate Custom|SpawnEnemy) 4.0 true false 0.0 1.0))

(event EventTick
  (params (DeltaSeconds :type Float%20%28single-precision%29))
  (Variables|Default|SetContador (+ DeltaSeconds (Variables|Default|GetContador))))

(fn ConstructionScript)