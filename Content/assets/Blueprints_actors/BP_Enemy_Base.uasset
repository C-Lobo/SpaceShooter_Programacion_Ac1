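; Base enemy actor for a shooter that flies along its initial forward vector, fires bullet spreads and dies on overlap.
; Tick moves it by Speed and fires whenever a timer re-arms FireTempo, fanning Bullet2 spawns in yaw from PointFire across AnguloDisparo.
; Overlaps tagged Player or Bullet_Player destroy it with explosion particles and sound, while Marco destroys it silently.
; A sine-wave movement function, MoveOnda, is defined but not called here.
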(event Custom|Fire_Update
  ;[1 1 1] Fire_Push
  (Variables|Default|SetFire_tempo true))

(event EventBeginPlay
  (Variables|Default|Setmovementvector (Transformation|GetActorForwardVector)))

(event Collision|EventActorBeginOverlap
  (params (OtherActor :type Actor%20Object%20Reference))
  ;[1 1 1] Overlap
  (if (Utilities|Array|ContainsItem (Variables|/Script/Engine.Actor|GetTags OtherActor) "Player")
    (Utilities|FlowControl|Delay 0.1)
    (Actor|DestroyActor)
    (CallFunction|ExplotionParticle :!label _label)
    (elif (Utilities|Array|ContainsItem (Variables|/Script/Engine.Actor|GetTags OtherActor) "Marco")
      (Utilities|FlowControl|Delay 0.1)
      (Actor|DestroyActor)
      (elif (Utilities|Array|ContainsItem (Variables|/Script/Engine.Actor|GetTags OtherActor) "Bullet_Player")
        (Utilities|FlowControl|Delay 0.08)
        (Actor|DestroyActor)
        (goto _label)))))

(event EventTick
  (params (DeltaSeconds :type Float%20%28single-precision%29))
  (CallFunction|MoveEnemy DeltaSeconds)
  ;[1 1 1] Fire_Push
  (if (Variables|Default|GetFire_tempo)
    (CallFunction|SpawBulletEnemy)
    (Variables|Default|SetFire_tempo false)
    (Utilities|Time|SetTimerbyEvent (delegate Custom|Fire_Update) (Variables|Default|GetTime_Bullet))))

(fn ConstructionScript)

(fn MoveEnemy
  (params (A :type Float%20%28double-precision%29))
  (Transformation|SetActorLocation (+ (Transformation|GetActorLocation) (* (* A (Variables|Default|GetSpeed)) (Variables|Default|Getmovementvector))) false false))

(fn MoveOnda
  (params (A :type Float%20%28double-precision%29) (A2 :type Float%20%28double-precision%29))
  (bind _speed (Variables|Default|GetSpeed))
  (bind _returnvalue (* A _speed))
  (Transformation|SetActorLocation (+ (Math|Vector|MakeVector _returnvalue (* (Math|Trig|Sin(Radians) (Utilities|Time|GetGameTimeinSeconds)) (Variables|Default|GetAmplitud)) 0.0) (+ (Transformation|GetActorLocation) (* _returnvalue (Variables|Default|Getmovementvector)))) false false))

(fn SpawBulletEnemy
  (for _index (range 0 (+ (Variables|Default|Getconunt) 0))
    (Game|SpawnActorfromClass "/Game/assets/Blueprints_actors/Bullet2.Bullet2_C" (Math|Transform|MakeTransform (.location (Transformation|GetWorldTransform (Variables|Default|GetPoint_fire))) (Math|Rotator|CombineRotators (Math|Rotator|MakeRotator 0.0 0.0 (.yaw (Transformation|GetSocketRotation (Variables|Default|GetPoint_fire) "None"))) (Math|Rotator|MakeRotator 0.0 0.0 (* _index (/ (Variables|Default|Getangulo_disparo) (Variables|Default|Getconunt))))) "1.000000,1.000000,1.000000") "AlwaysSpawn" "MultiplyWithRoot" 0 0)))

(fn ExplotionParticle
  (Effects|SpawnEmitteratLocation "/Game/Weapons/Plasma/P_Orb_Explosion.P_Orb_Explosion" (Transformation|GetActorLocation))
  (Effects|SpawnEmitteratLocation "/Game/FX/Character/P_HitEffectGeneric.P_HitEffectGeneric" (Transformation|GetActorLocation))
  (Audio|PlaySound2D "/Game/StarterContent/Audio/Explosion02.Explosion02" 1.0 1.0 0.0 0 0))